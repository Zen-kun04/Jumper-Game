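; BP_BaseCharacter is a player character with Enhanced Input movement, mouse look, jumping, footstep audio and a coin counter.
; BeginPlay adds the default mapping context and shows the WB_Coins widget.
; Forward-axis input sets IsWalking above a horizontal speed threshold and clears it on release, while Tick starts or stops FootstepAudioComponent to match; strafing leaves the flag untouched.
; GetCoins and IncrementCoins expose the coin count.
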(event Input|EnhancedActionEvents|EnhancedInputActionIA_X
  (params (ActionValue :type Vector%202D%20Structure) (ElapsedSeconds :type Float%20%28double-precision%29) (TriggeredSeconds :type Float%20%28double-precision%29) (InputAction :type Input%20Action%20Object%20Reference :default "/Game/InputActions/IA_X.IA_X"))
  (:Triggered
    (Pawn|Input|AddMovementInput (Transformation|GetActorForwardVector) (.x ActionValue) false)
    (if (> (Math|Vector|VectorLengthXY (Transformation|GetVelocity)) 2e+02)
      (Variables|Default|SetIsWalking true)))
  (:Canceled
    (Variables|Default|SetIsWalking false :!label _label))
  (:Completed
    (goto _label)))

(event Input|EnhancedActionEvents|EnhancedInputActionIA_Y
  (params (ActionValue :type Vector%202D%20Structure) (ElapsedSeconds :type Float%20%28double-precision%29) (TriggeredSeconds :type Float%20%28double-precision%29) (InputAction :type Input%20Action%20Object%20Reference :default "/Game/InputActions/IA_Y.IA_Y"))
  (Pawn|Input|AddMovementInput (Transformation|GetActorRightVector) (.X (Math|Vector2D|BreakVector2D ActionValue)) false))

(event Input|EnhancedActionEvents|EnhancedInputActionIA_Mouse
  (params (ActionValue :type Vector%202D%20Structure) (ElapsedSeconds :type Float%20%28double-precision%29) (TriggeredSeconds :type Float%20%28double-precision%29) (InputAction :type Input%20Action%20Object%20Reference :default "/Game/InputActions/IA_Mouse.IA_Mouse"))
  (Pawn|Input|AddControllerPitchInput (.y ActionValue))
  (Pawn|Input|AddControllerYawInput (.x ActionValue)))

(event Input|EnhancedActionEvents|EnhancedInputActionIA_Jump
  (params (ActionValue :type Boolean) (ElapsedSeconds :type Float%20%28double-precision%29) (TriggeredSeconds :type Float%20%28double-precision%29) (InputAction :type Input%20Action%20Object%20Reference :default "/Game/InputActions/IA_Jump.IA_Jump"))
  (Character|Jump))

(event EventBeginPlay
  (Input|AddMappingContext (PlayerController|LocalPlayerSubsystems|GetEnhancedInputLocalPlayerSubsystem (Game|GetPlayerController 0)) "/Game/InputActions/IMC_Default.IMC_Default" 0 "(bIgnoreAllPressedKeysUntilRelease=True,bForceImmediately=False,bNotifyUserSettings=False)")
  (bind _returnvalue (UserInterface|CreateWidget "/Game/WB_Coins.WB_Coins_C"))
  (UserInterface|Viewport|AddtoViewport _returnvalue 0))

(event Collision|EventActorBeginOverlap
  (params (OtherActor :type Actor%20Object%20Reference)))

(event EventTick
  (params (DeltaSeconds :type Float%20%28single-precision%29))
  (bind _footstepaudiocomponent (Variables|Default|GetFootstepAudioComponent))
  (Utilities|FlowControl|Sequence
    (:then_0
      (if (and (Variables|Default|GetIsWalking) (!= (Variables|Default|GetIsPlayingSound) true))
        (Variables|Default|SetIsPlayingSound true)
        (Audio|Components|Audio|Play _footstepaudiocomponent 0.0)))
    (:then_1
      (if (and (!= (Variables|Default|GetIsWalking) true) (Variables|Default|GetIsPlayingSound))
        (Variables|Default|SetIsPlayingSound false)
        (Audio|Components|Audio|Stop _footstepaudiocomponent)))))

(fn ConstructionScript)

(fn GetCoins
  (return (Variables|Default|Getcoins)))

(fn IncrementCoins
  (Variables|Default|Setcoins (+ (Variables|Default|Getcoins) 1)))